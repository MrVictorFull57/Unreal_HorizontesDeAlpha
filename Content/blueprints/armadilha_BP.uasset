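; A fire trap that alternates between idle and flaming, damaging the alpha_BP protagonist on contact.
; A timer triggers each burst with sound, particles, a light and the Box collision, then a delay shuts them off and restarts the timer.
; Box overlap sends a damage struct and flags the player as inside the damage area, clearing that flag after a short delay or when the burst ends.
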(event OnComponentBeginOverlap(Box)
  (params (OverlappedComponent :type Primitive%20Component%20Object%20Reference) (OtherActor :type Actor%20Object%20Reference) (OtherComp :type Primitive%20Component%20Object%20Reference) (OtherBodyIndex :type Integer) (bFromSweep :type Boolean) (SweepResult :type Hit%20Result%20Structure%20%28by%20ref%29))
  (bind _asalpha_bp (Utilities|Casting|CastToalpha_BP OtherActor))
  (bind _output_get (Variables|Default|SetAs%20Bp%20Protagonista%20Alpha _asalpha_bp))
  (Default|AreaDano _output_get)
  (Class|BpiSistemaDano|LevaDano(Message) _output_get (Utilities|Struct|Makes_info_dano 1e+01 "NewEnumerator1" "NewEnumerator1"))
  (Utilities|FlowControl|Delay 0.8)
  (bind _as_bp_protagonista_alpha (Variables|Default|GetAs%20Bp%20Protagonista%20Alpha)
    (:then
      (Default|ForaAreaDano _as_bp_protagonista_alpha))
    (:else)))

(event Custom|ativa_armadilha
  (bind _returnvalue (Utilities|Time|SetTimerbyEvent (delegate Custom|timer_fogo) 3.0 true))
  (Variables|Default|SetTempo _returnvalue))

(event Custom|timer_fogo
  (bind _staticmesh (Variables|Default|GetStaticMesh))
  (bind _returnvalue (Transformation|GetWorldLocation _staticmesh))
  (Audio|PlaySoundatLocation "/Game/sons/labareda_armadilha.labareda_armadilha" _returnvalue "0, 0, 0" 1.0 1.0 0.0 "/Game/sons/atenuação_sons.atenuação_sons" 0 0 0)
  (bind _returnvalue_2 (Effects|SpawnEmitteratLocation "/Game/vfx/particulas/fogo_ptc.fogo_ptc" _returnvalue))
  (Rendering|SetVisibility (Variables|Default|GetPointLight) true false)
  (Collision|SetCollisionEnabled (Variables|Default|GetBox) "QueryAndPhysics")
  (Utilities|FlowControl|Delay 3.0)
  (Components|DestroyComponent _returnvalue_2)
  (Rendering|SetVisibility (Variables|Default|GetPointLight) false false)
  (Collision|SetCollisionEnabled (Variables|Default|GetBox) "NoCollision")
  (Utilities|Time|ClearandInvalidateTimerbyHandle (Variables|Default|GetTempo))
  (CallFunction|AtivaArmadilha)
  (bind _as_bp_protagonista_alpha (Variables|Default|GetAs%20Bp%20Protagonista%20Alpha)
    (:then
      (Default|ForaAreaDano _as_bp_protagonista_alpha))
    (:else)))

(event EventBeginPlay
  (Collision|SetCollisionEnabled (Variables|Default|GetBox) "NoCollision")
  (CallFunction|AtivaArmadilha))

(fn ConstructionScript)