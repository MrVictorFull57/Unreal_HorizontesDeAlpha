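; Game instance that holds player progress: stage and Stella unlocks, records, best grades, button style, music setting and a running score.
; Init copies values from the save slot, and salva_progresso writes them into a fresh save object after a short delay.
; apaga_progresso deletes the slot, resets stage progress, plays a sound, briefly mutes menu music and shows a temporary hint widget.
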(event Custom|apaga_progresso
  (SaveGame|DeleteGameinSlot "slot_do_player")
  (Development|PrintString "Progresso das Fases foi Apagado.")
  (Audio|PlaySound2D "/Game/sons/menu/save_apagado.save_apagado" 1.0 1.0 0.0 0 0)
  (Variables|Default|SetFase2Liberada false)
  (Variables|Default|SetFase3Liberada false)
  (Variables|Default|SetStellaLiberada false)
  (Variables|Default|SetPontoRecordeFase1 0)
  (Variables|Default|SetPontoRecordeFase2 0)
  (Variables|Default|SetPontoRecordeFase3 0)
  (Variables|Default|SetMelhorNotaFase1 0)
  (Variables|Default|SetMelhorNotaFase2 0)
  (Variables|Default|SetMelhorNotaFase3 0)
  (Utilities|FlowControl|Sequence
    (:then_0
      (bind _outactors (Actor|GetAllActorsOfClass "/Game/blueprints/musica_menu.musica_menu_C"))
      (Audio|Components|Audio|SetVolumeMultiplier (Variables|/Game/blueprints/musica_menu.musica_menu_C|Getmenu-2 (Utilities|Array|Get(acopy) _outactors)) 0.0 :!class /Script/Engine.AudioComponent)
      (Utilities|FlowControl|Delay 1.5)
      (Audio|Components|Audio|SetVolumeMultiplier (Variables|/Game/blueprints/musica_menu.musica_menu_C|Getmenu-2 (Utilities|Array|Get(acopy) _outactors)) 1.0 :!class /Script/Engine.AudioComponent))
    (:then_1
      (bind _returnvalue (UserInterface|CreateWidget "/Game/ui/hint_progresso_apagado.hint_progresso_apagado_C"))
      (UserInterface|Viewport|AddtoViewport _returnvalue 0)
      (Utilities|FlowControl|Delay 1.6)
      (Widget|RemovefromParent _returnvalue))))

(event Custom|salva_progresso
  (Utilities|FlowControl|Delay 0.2)
  (bind _returnvalue (SaveGame|CreateSaveGameObject "/Game/blueprints/SaveProgresso_BP.SaveProgresso_BP_C"))
  (Variables|/Game/blueprints/SaveProgresso_BP.SaveProgresso_BP_C|SetFase2Liberada _returnvalue (Variables|Default|GetFase2Liberada))
  (Variables|/Game/blueprints/SaveProgresso_BP.SaveProgresso_BP_C|SetFase3Liberada _returnvalue (Variables|Default|GetFase3Liberada))
  (Variables|/Game/blueprints/SaveProgresso_BP.SaveProgresso_BP_C|SetStellaLiberada _returnvalue (Variables|Default|GetStellaLiberada))
  (Variables|/Game/blueprints/SaveProgresso_BP.SaveProgresso_BP_C|SetPontoRecordeFase1 _returnvalue (Variables|Default|GetPontoRecordeFase1))
  (Variables|/Game/blueprints/SaveProgresso_BP.SaveProgresso_BP_C|SetPontoRecordeFase2 _returnvalue (Variables|Default|GetPontoRecordeFase2))
  (Variables|/Game/blueprints/SaveProgresso_BP.SaveProgresso_BP_C|SetPontoRecordeFase3 _returnvalue (Variables|Default|GetPontoRecordeFase3))
  (Variables|/Game/blueprints/SaveProgresso_BP.SaveProgresso_BP_C|SetMelhorNotaFase1 _returnvalue (Variables|Default|GetMelhorNotaFase1))
  (Variables|/Game/blueprints/SaveProgresso_BP.SaveProgresso_BP_C|SetMelhorNotaFase2 _returnvalue (Variables|Default|GetMelhorNotaFase2))
  (Variables|/Game/blueprints/SaveProgresso_BP.SaveProgresso_BP_C|SetMelhorNotaFase3 _returnvalue (Variables|Default|GetMelhorNotaFase3))
  (Variables|/Game/blueprints/SaveProgresso_BP.SaveProgresso_BP_C|SetBotaoEstiloAtual _returnvalue (Variables|Default|GetBotaoEstiloAtual))
  (Variables|/Game/blueprints/SaveProgresso_BP.SaveProgresso_BP_C|SetMusicasLigadas _returnvalue (Variables|Default|GetMusicasLigadas))
  (SaveGame|SaveGametoSlot _returnvalue "slot_do_player")
  (Development|PrintString "Progresso foi Salvo."))

(event EventInit
  (bind _returnvalue (SaveGame|LoadGamefromSlot "slot_do_player"))
  (Utilities|IsValid _returnvalue
    (:Is%20Valid
      (bind _assave_progresso_bp (Utilities|Casting|CastToSaveProgresso_BP _returnvalue))
      (Variables|Default|SetFase2Liberada (Variables|/Game/blueprints/SaveProgresso_BP.SaveProgresso_BP_C|GetFase2Liberada _assave_progresso_bp))
      (Variables|Default|SetFase3Liberada (Variables|/Game/blueprints/SaveProgresso_BP.SaveProgresso_BP_C|GetFase3Liberada _assave_progresso_bp))
      (Variables|Default|SetStellaLiberada (Variables|/Game/blueprints/SaveProgresso_BP.SaveProgresso_BP_C|GetStellaLiberada _assave_progresso_bp))
      (Variables|Default|SetBotaoEstiloAtual (Variables|/Game/blueprints/SaveProgresso_BP.SaveProgresso_BP_C|GetBotaoEstiloAtual _assave_progresso_bp))
      (Variables|Default|SetMusicasLigadas (Variables|/Game/blueprints/SaveProgresso_BP.SaveProgresso_BP_C|GetMusicasLigadas _assave_progresso_bp))
      (Variables|Default|SetPontoRecordeFase1 (Variables|/Game/blueprints/SaveProgresso_BP.SaveProgresso_BP_C|GetPontoRecordeFase1 _assave_progresso_bp))
      (Variables|Default|SetPontoRecordeFase2 (Variables|/Game/blueprints/SaveProgresso_BP.SaveProgresso_BP_C|GetPontoRecordeFase2 _assave_progresso_bp))
      (Variables|Default|SetPontoRecordeFase3 (Variables|/Game/blueprints/SaveProgresso_BP.SaveProgresso_BP_C|GetPontoRecordeFase3 _assave_progresso_bp))
      (Variables|Default|SetMelhorNotaFase1 (Variables|/Game/blueprints/SaveProgresso_BP.SaveProgresso_BP_C|GetMelhorNotaFase1 _assave_progresso_bp))
      (Variables|Default|SetMelhorNotaFase2 (Variables|/Game/blueprints/SaveProgresso_BP.SaveProgresso_BP_C|GetMelhorNotaFase2 _assave_progresso_bp))
      (Variables|Default|SetMelhorNotaFase3 (Variables|/Game/blueprints/SaveProgresso_BP.SaveProgresso_BP_C|GetMelhorNotaFase3 _assave_progresso_bp)))))

(fn AdicionaPontuação
  (params (Quantia :type Integer))
  (Variables|Default|SetPontos (+ Quantia (Variables|Default|GetPontos)))
  (return))