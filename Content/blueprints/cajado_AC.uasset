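; Staff combat component for the protagonist Character, handling equipping, aiming and shooting animation.
; On BeginPlay it caches the owning Character, spawns the staff Blueprint and snaps it to a mesh socket.
; Aiming switches rotation from movement-oriented to controller-driven.
; Shooting requires aiming and plays a montage behind a DoOnce that resets on completion or interruption, then reapplies aim; the shooting flag is never set back to false.
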(event Custom|ParaMIra
  (bind _referênciaprotagonista (Variables|Default|GetReferênciaProtagonista))
  (bind _charactermovement (Variables|/Script/Engine.Character|GetCharacterMovement _referênciaprotagonista))
  (Variables|Default|SetEstáMirando false)
  (Variables|/Script/Engine.CharacterMovementComponent|SetbOrientRotationToMovement _charactermovement true)
  (Variables|/Script/Engine.CharacterMovementComponent|SetbUseControllerDesiredRotation _charactermovement false))

(event Custom|ComeçaMira
  (bind _referênciaprotagonista (Variables|Default|GetReferênciaProtagonista))
  (bind _charactermovement (Variables|/Script/Engine.Character|GetCharacterMovement _referênciaprotagonista))
  (Variables|Default|SetEstáMirando true)
  (Variables|/Script/Engine.CharacterMovementComponent|SetbOrientRotationToMovement _charactermovement false)
  (Variables|/Script/Engine.CharacterMovementComponent|SetbUseControllerDesiredRotation _charactermovement true))

(event Custom|TiroFim
  (Variables|Default|SetEstáAtirando true)
  (if (Variables|Default|GetEstáMirando)
    (CallFunction|ComeçaMira)))

(event Custom|TiroComeço
  (if (Variables|Default|GetEstáMirando)
    (Variables|Default|SetEstáAtirando true)
    (Utilities|FlowControl|DoOnce false :!label _label
      (:Completed
        (Animation|Montage|PlayMontage (Variables|/Script/Engine.Character|GetMesh (Variables|Default|GetReferênciaProtagonista)) (Variables|Default|GetAtirando_Montage)
          (:OnCompleted
            _)
          (:OnInterrupted
            _))
        (CallFunction|TiroFim)
        (goto _label Reset)))))

(event EventBeginPlay
  (bind _ascharacter (Utilities|Casting|CastToCharacter (Components|GetOwner)))
  (Variables|Default|SetReferênciaProtagonista _ascharacter)
  (CallFunction|EquipaCajado))

(fn EquipaCajado
  (bind _returnvalue (Game|SpawnActorfromClass (Variables|Default|Getcajado_BP) (Math|Transform|MakeTransform "0, 0, 0" "0, 0, 0" "1.000000,1.000000,1.000000") "Undefined" "MultiplyWithRoot" 0 0))
  (Transformation|AttachComponentToComponent _returnvalue (Variables|/Script/Engine.Character|GetMesh (Variables|Default|GetReferênciaProtagonista)) (Variables|Default|GetNomeSocketCajado) "SnapToTarget" "SnapToTarget" "SnapToTarget" true))