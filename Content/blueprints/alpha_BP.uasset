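; Player character Blueprint for the protagonist Alpha, with Enhanced Input movement, swimming, melee, aimed staff shots, chest opening and pause.
; Timelines drive first/third-person switching, aim zoom and the victory camera.
; BpcSistemaDano handles health and combat callbacks, while looping timers refresh the health bar and low-health sound.
; Death and hazard falls detach the camera and show Game Over; Respawn restores the checkpoint, deducts points and heals the boss.
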(event Custom|TocaSomVidaBaixa
  ;[1 1 1] toca um som quando a vida estiver baixa
  (Utilities|FlowControl|Sequence
    (:then_0
      (if (<= (Variables|/Game/sistema_dano/bpc_sistema_dano.bpc_sistema_dano_C|GetVida (Variables|Default|Getbpc_sistema_dano)) (Variables|Default|GetLimiteVidaBaixa))
        (if (not (Variables|Default|GetTocouSomVidaBaixa))
          (Audio|PlaySound2D "/Game/sons/vida-baixa.vida-baixa" 1.0 1.0 0.0 0 0)
          (Variables|Default|SetTocouSomVidaBaixa true))))
    (:then_1
      (if (> (Variables|/Game/sistema_dano/bpc_sistema_dano.bpc_sistema_dano_C|GetVida (Variables|Default|Getbpc_sistema_dano)) (Variables|Default|GetLimiteVidaBaixa))
        (Variables|Default|SetTocouSomVidaBaixa false)))))

(event Custom|Fora_Area_Dano
  ;[1 1 1] verifica armadilha
  (Variables|Default|SetSofrer_dano false))

(event Custom|VenceuLevel
  (bind _springarm (Variables|Camera|GetSpringArm))
  ;[1 1 1] vitória
  (Utilities|FlowControl|Delay 0.8)
  (Input|DisableInput (Game|GetPlayerController 0))
  (Transformation|SetActorRotation (Math|Rotator|FindLookatRotation (Transformation|GetActorLocation) (Transformation|GetWorldLocation (Variables|Camera|GetCamera))))
  (bind _miraalpha (Timeline|Timeline Play)
    (:Update
      (Camera|SetFieldOfView (Variables|Camera|GetCamera) (Math|Float|Lerp (Variables|Default|GetNormalPOV) (Variables|Default|GetVitoriaPOV) _miraalpha))
      (Variables|/Script/Engine.SpringArmComponent|SetSocketOffset _springarm (Math|Vector|Lerp(Vector) (Variables|Default|GetNormalBoom) (Variables|Default|GetVitoriaBoom) _miraalpha))
      (Variables|/Script/Engine.SpringArmComponent|SetbInheritPitch _springarm false)
      (bind _outactors (Actor|GetAllActorsOfClass "/Game/blueprints/musica_fase.musica_fase_C"))
      (Audio|Components|Audio|FadeOut (Variables|/Game/blueprints/musica_fase.musica_fase_C|Getfase (Utilities|Array|Get(acopy) _outactors)) 1.0 0.0 "Linear" :!class /Script/Engine.AudioComponent)
      (Utilities|FlowControl|Delay 1.0)
      (Audio|Components|Audio|Stop (Variables|/Game/blueprints/musica_fase.musica_fase_C|Getfase (Utilities|Array|Get(acopy) _outactors)))
      (Viewport|RemoveAllWidgets)
      (Components|Animation|PlayAnimation (Variables|Character|GetMesh) "/Game/animacoes/alpha/venceu.venceu" false)
      (Audio|PlaySound2D "/Game/musicas/vitória2.vitória2" 1.0 1.0 0.0 0 0)
      (Audio|PlaySoundatLocation "/Game/sons/vozes/alpha_voz_venceu.alpha_voz_venceu" (Transformation|GetActorLocation) "0, 0, 0" 1.0 1.0 0.0 0 0 0 0)
      (Utilities|FlowControl|Delay 1.0)
      (bind _returnvalue (UserInterface|CreateWidget "/Game/menus/menu_Vitoria.menu_Vitoria_C" (Game|GetPlayerController 0)))
      (UserInterface|Viewport|AddtoViewport _returnvalue 2))))

(event Custom|IniciaVariáveis
  ;[1 1 1] define visão inicial
  (Variables|Default|SetNormalPOV (Variables|/Script/Engine.CameraComponent|GetFieldOfView (Variables|Camera|GetCamera)))
  (Variables|Default|SetNormalBoom (Variables|/Script/Engine.SpringArmComponent|GetSocketOffset (Variables|Camera|GetSpringArm))))

(event Custom|caiu_no_buraco
  ;[1 1 1] cai no buraco
  (Components|Activation|Deactivate (Variables|Default|GetPrimeiraPessoa))
  (Components|Activation|Activate (Variables|Camera|GetCamera) true)
  (Variables|Default|SetbUseControllerRotationYaw false)
  (Utilities|FlowControl|DoOnce false :!label _label
    (:Completed
      (Development|PrintString "ADEUS MUNDO CRUEL")
      (Transformation|DetachFromComponent (Variables|Camera|GetSpringArm) "KeepWorld" "KeepWorld" "KeepWorld" true)
      (Input|DisableInput (Game|GetPlayerController 0))
      (Audio|PlaySoundatLocation (Variables|Default|GetVozGritoQueda) (Transformation|GetActorLocation) "0, 0, 0" 1.0 1.0 0.0 0 0 0 0)
      (bind _outactors (Actor|GetAllActorsOfClass "/Game/blueprints/musica_fase.musica_fase_C"))
      (Default|MusicaFicouLenta (Utilities|Array|Get(acopy) _outactors))
      (Utilities|FlowControl|Delay 2.6)
      (if (not (Variables|Default|GetJáTáMorta))
        (bind _returnvalue (UserInterface|CreateWidget "/Game/menus/menu_GameOver.menu_GameOver_C" (Game|GetPlayerController 0)))
        (Variables|Default|SetJáTáMorta true)
        (UserInterface|Viewport|AddtoViewport _returnvalue 2)
        (goto _label Reset)))))

(event Custom|caiu_na_agua
  (bind _mesh (Variables|Character|GetMesh))
  (bind _returnvalue (Transformation|GetSocketLocation _mesh "RightFoot"))
  ;[1 1 1] cai na água
  (Components|Activation|Deactivate (Variables|Default|GetPrimeiraPessoa))
  (Components|Activation|Activate (Variables|Camera|GetCamera) true)
  (Variables|Default|SetbUseControllerRotationYaw false)
  (Utilities|FlowControl|DoOnce false :!label _label
    (:Completed
      (Development|PrintString "TO AFOGADO")
      (Niagara|SpawnSystematLocation "/Game/vfx/particulas_2/tibum-de-agua-NS.tibum-de-agua-NS" _returnvalue)
      (Transformation|DetachFromComponent (Variables|Camera|GetSpringArm) "KeepWorld" "KeepWorld" "KeepWorld" true)
      (Input|DisableInput (Game|GetPlayerController 0))
      (Audio|PlaySoundatLocation "/Game/sons/cues/voz_afoga_cue.voz_afoga_cue" _returnvalue "0, 0, 0" 1.0 1.0 0.0 0 0 0 0)
      (bind _outactors (Actor|GetAllActorsOfClass "/Game/blueprints/musica_fase.musica_fase_C"))
      (Default|MusicaFicouLenta (Utilities|Array|Get(acopy) _outactors))
      (Utilities|FlowControl|Delay 2.6)
      (if (not (Variables|Default|GetJáTáMorta))
        (bind _returnvalue_2 (UserInterface|CreateWidget "/Game/menus/menu_GameOver.menu_GameOver_C" (Game|GetPlayerController 0)))
        (Variables|Default|SetJáTáMorta true)
        (UserInterface|Viewport|AddtoViewport _returnvalue_2 2)
        (goto _label Reset)))))

(event Custom|para_de_nadar
  (bind _charactermovement (Variables|Character|GetCharacterMovement))
  (Pawn|Components|CharacterMovement|SetMovementMode _charactermovement "MOVE_Walking" 0)
  (Variables|Default|SetEstáNadando false)
  (Variables|/Script/Engine.CharacterMovementComponent|SetGravityScale _charactermovement 1.75))

(event Custom|começa_a_nadar
  (bind _charactermovement (Variables|Character|GetCharacterMovement))
  (Pawn|Components|CharacterMovement|SetMovementMode _charactermovement "MOVE_Swimming" 0)
  (Variables|Default|SetEstáNadando true)
  (Variables|/Script/Engine.CharacterMovementComponent|SetGravityScale _charactermovement 0.44))

(event Custom|Area_Dano
  ;[1 1 1] verifica armadilha
  (Variables|Default|SetSofrer_dano true)
  (Utilities|FlowControl|DoOnce false :!label _label
    (:Completed
      (Pawn|Components|CharacterMovement|SetMovementMode (Variables|Character|GetCharacterMovement) "MOVE_None" 0)
      (Animation|PlayAnimMontage (Variables|Default|GetAnimDeLevarDano) 1.0 "None")
      (Utilities|FlowControl|Delay 0.55)
      (Pawn|Components|CharacterMovement|SetMovementMode (Variables|Character|GetCharacterMovement) "MOVE_Walking" 0)
      (bind _asmodo_de_jogo_principal_alpha (Utilities|Casting|CastTomodoDeJogoPrincipal_alpha (Game|GetGameMode)))
      (Default|AtualizaBarraRed (Variables|/Game/blueprints/modoDeJogoPrincipal_alpha.modoDeJogoPrincipal_alpha_C|GetBarraVidaUI _asmodo_de_jogo_principal_alpha))
      (goto _label Reset))))

(event Custom|Esta_na_area
  (params (bau :type Bau%20Cristal%20BP%20Object%20Reference))
  ;[1 1 1] checa se está na area do baú
  (Variables|Default|SetBau bau)
  (Variables|Default|SetEsta_na_area_bau true))

(event Custom|nao_Esta_na_area
  (params (bau :type Bau%20Cristal%20BP%20Object%20Reference))
  ;[1 1 1] checa se está na area do baú
  (Variables|Default|SetBau bau)
  (Variables|Default|SetEsta_na_area_bau false))

(event Custom|atualiza_vida_verm
  (bind _asmodo_de_jogo_principal_alpha (Utilities|Casting|CastTomodoDeJogoPrincipal_alpha (Game|GetGameMode)))
  (Utilities|IsValid (Variables|/Game/blueprints/modoDeJogoPrincipal_alpha.modoDeJogoPrincipal_alpha_C|GetBarraVidaUI _asmodo_de_jogo_principal_alpha)
    (:Is%20Valid
      (Default|AtualizaBarraRed (Variables|/Game/blueprints/modoDeJogoPrincipal_alpha.modoDeJogoPrincipal_alpha_C|GetBarraVidaUI _asmodo_de_jogo_principal_alpha)))))

(event Custom|caiu_na_lava
  (Components|Activation|Deactivate (Variables|Default|GetPrimeiraPessoa))
  (Components|Activation|Activate (Variables|Camera|GetCamera) true)
  (Variables|Default|SetbUseControllerRotationYaw false)
  (Utilities|FlowControl|DoOnce false :!label _label
    (:Completed
      (Development|PrintString "PUTA VIDA")
      (Effects|SpawnEmitteratLocation "/Game/StarterContent/Particles/P_Explosion.P_Explosion" (Transformation|GetSocketLocation (Variables|Character|GetMesh) "Spine") "0, 0, 0" "1.800000,1.800000,1.800000")
      (Transformation|DetachFromComponent (Variables|Camera|GetSpringArm) "KeepWorld" "KeepWorld" "KeepWorld" true)
      (Input|DisableInput (Game|GetPlayerController 0))
      (bind _outactors (Actor|GetAllActorsOfClass "/Game/blueprints/musica_fase.musica_fase_C"))
      (Default|MusicaFicouLenta (Utilities|Array|Get(acopy) _outactors))
      (Utilities|FlowControl|Delay 2.6)
      (if (not (Variables|Default|GetJáTáMorta))
        (bind _returnvalue (UserInterface|CreateWidget "/Game/menus/menu_GameOver.menu_GameOver_C" (Game|GetPlayerController 0)))
        (Variables|Default|SetJáTáMorta true)
        (UserInterface|Viewport|AddtoViewport _returnvalue 2)
        (goto _label Reset)))))

(event Custom|CâmeraMiraFim
  ;[1 1 1] sistema de mira em 3ª pessoa
  (bind _miraalpha (Timeline|TimelineCameraMira Reverse)
    (:Update
      (Camera|SetFieldOfView (Variables|Camera|GetCamera) (Math|Float|Lerp (Variables|Default|GetNormalPOV) (Variables|Default|GetMiraPOV) _miraalpha))
      (Variables|/Script/Engine.SpringArmComponent|SetSocketOffset (Variables|Camera|GetSpringArm) (Math|Vector|Lerp(Vector) (Variables|Default|GetNormalBoom) (Variables|Default|GetMiraBoom) _miraalpha)))))

(event Custom|Morreu
  ;[1 1 1] morte
  (Utilities|FlowControl|DoOnce false :!label _label
    (:Completed
      (Development|PrintString "MORRI, QUE MERDA...")
      (Transformation|DetachFromComponent (Variables|Camera|GetSpringArm) "KeepWorld" "KeepWorld" "KeepWorld" true)
      (Input|DisableInput (Game|GetPlayerController 0))
      (Components|Animation|PlayAnimation (Variables|Character|GetMesh) "/Game/animacoes/alpha/morre.morre" false)
      (Audio|PlaySoundatLocation "/Game/sons/vozes/alpha_voz_morte.alpha_voz_morte" (Transformation|GetActorLocation) "0, 0, 0" 1.0 1.0 0.0 0 0 0 0)
      (bind _outactors (Actor|GetAllActorsOfClass "/Game/blueprints/musica_fase.musica_fase_C"))
      (Default|MusicaFicouLenta (Utilities|Array|Get(acopy) _outactors))
      (Utilities|Time|SetGlobalTimeDilation 0.2)
      (Utilities|FlowControl|Delay 0.03)
      (Utilities|Time|SetGlobalTimeDilation 1.0)
      (Utilities|FlowControl|Delay 1.5)
      (Utilities|FlowControl|Delay 1.0)
      (if (not (Variables|Default|GetJáTáMorta))
        (bind _returnvalue (UserInterface|CreateWidget "/Game/menus/menu_GameOver.menu_GameOver_C" (Game|GetPlayerController 0)))
        (Variables|Default|SetJáTáMorta true)
        (UserInterface|Viewport|AddtoViewport _returnvalue 2)
        (goto _label Reset)))))

(event Custom|Bloqueou
  (params (PodeDarParry :type Boolean))
  (Development|PrintString "DEU PARRY!"))

(event Custom|RespostaAoDano
  (params (RespostaAoDano :type e_resposta_dano%20Enum :default "NewEnumerator0"))
  (Development|PrintString (Utilities|String|EnumtoString RespostaAoDano)))

(event Custom|CâmeraMiraComeço
  ;[1 1 1] sistema de mira em 3ª pessoa
  (bind _miraalpha (Timeline|TimelineCameraMira Play)
    (:Update
      (Camera|SetFieldOfView (Variables|Camera|GetCamera) (Math|Float|Lerp (Variables|Default|GetNormalPOV) (Variables|Default|GetMiraPOV) _miraalpha))
      (Variables|/Script/Engine.SpringArmComponent|SetSocketOffset (Variables|Camera|GetSpringArm) (Math|Vector|Lerp(Vector) (Variables|Default|GetNormalBoom) (Variables|Default|GetMiraBoom) _miraalpha)))))

(event Input|EnhancedActionEvents|EnhancedInputActionia_movimentar
  (params (ActionValue :type Vector%202D%20Structure) (ElapsedSeconds :type Float%20%28double-precision%29) (TriggeredSeconds :type Float%20%28double-precision%29) (InputAction :type Input%20Action%20Object%20Reference :default "/Game/inputs/ia_movimentar.ia_movimentar"))
  (bind _returnvalue (Pawn|GetControlRotation :!class /Script/Engine.Pawn))
  ;[1 1 1] se movimenta
  ;;[1 1 1] esquerda e direita
  (Pawn|Input|AddMovementInput (Math|Vector|GetRightVector (Math|Rotator|MakeRotator (.roll _returnvalue) 0.0 (.yaw _returnvalue))) (.x ActionValue) false)
  ;;[1 1 1] pra frente e pra tras
  (Pawn|Input|AddMovementInput (Math|Vector|GetForwardVector (Math|Rotator|MakeRotator 0.0 0.0 (.yaw (Pawn|GetControlRotation :!class /Script/Engine.Pawn)))) (.y ActionValue) false))

(event Input|EnhancedActionEvents|EnhancedInputActionia_olhar
  (params (ActionValue :type Vector%202D%20Structure) (ElapsedSeconds :type Float%20%28double-precision%29) (TriggeredSeconds :type Float%20%28double-precision%29) (InputAction :type Input%20Action%20Object%20Reference :default "/Game/inputs/ia_olhar.ia_olhar"))
  ;[1 1 1] mexe a camera
  (Pawn|Input|AddControllerYawInput (.x ActionValue))
  (Pawn|Input|AddControllerPitchInput (.y ActionValue)))

(event Input|EnhancedActionEvents|EnhancedInputActionia_pular
  (params (ActionValue :type Boolean) (ElapsedSeconds :type Float%20%28double-precision%29) (TriggeredSeconds :type Float%20%28double-precision%29) (InputAction :type Input%20Action%20Object%20Reference :default "/Game/inputs/ia_pular.ia_pular"))
  ;[1 1 1] pular (ou subir ao nadar)
  (:Started
    (if (Variables|Default|GetEstáNadando)
      (Character|LaunchCharacter "0.000000,0.000000,500.000000" false true)
      (Audio|PlaySound2D "/Game/sons/nadando.nadando" 1.0 1.0 0.0 0 0)
      (Utilities|FlowControl|Delay 0.1)
      (Pawn|Components|CharacterMovement|SetMovementMode (Variables|Character|GetCharacterMovement) "MOVE_Swimming" 0)
      (else
        (Character|Jump))))
  (:Completed
    (Character|StopJumping)))

(event Input|EnhancedActionEvents|EnhancedInputActionia_atacar
  (params (ActionValue :type Boolean) (ElapsedSeconds :type Float%20%28double-precision%29) (TriggeredSeconds :type Float%20%28double-precision%29) (InputAction :type Input%20Action%20Object%20Reference :default "/Game/inputs/ia_atacar.ia_atacar"))
  (bind _animaçõesdeataque (Variables|Default|GetAnimaçõesDeAtaque))
  ;[1 1 1] atacando
  (if (not (Variables|Default|GetAtirando))
    (if (not (Variables|/Game/blueprints/cajado_AC.cajado_AC_C|GetEstáMirando (Actor|GetComponentbyClass "/Game/blueprints/cajado_AC.cajado_AC_C")))
      (Utilities|FlowControl|DoOnce false :!label _label
        (:Completed
          (Animation|PlayAnimMontage (Utilities|Array|Get(acopy) _animaçõesdeataque (Math|Random|RandomInteger (Utilities|Array|Length _animaçõesdeataque))) 1.2 "None")
          (Utilities|FlowControl|Delay 0.9)
          (goto _label Reset))))))

(event Input|EnhancedActionEvents|EnhancedInputActionia_abrir
  (params (ActionValue :type Boolean) (ElapsedSeconds :type Float%20%28double-precision%29) (TriggeredSeconds :type Float%20%28double-precision%29) (InputAction :type Input%20Action%20Object%20Reference :default "/Game/inputs/ia_abrir.ia_abrir"))
  ;[1 1 1] abre um báu
  (if (Variables|Default|GetEsta_na_area_bau)
    (Pawn|Components|CharacterMovement|SetMovementMode (Variables|Character|GetCharacterMovement) "MOVE_None" 0)
    (Utilities|FlowControl|DoOnce false :!label _label
      (:Completed
        (Animation|PlayAnimMontage (Variables|Default|GetAnimDeAbrirBaú) 1.2 "None")
        (Utilities|FlowControl|Delay 1.0)
        (bind _bau (Variables|Default|GetBau)
          (:then
            (Default|AnimAbrirBau _bau)
            (Pawn|Components|CharacterMovement|SetMovementMode (Variables|Character|GetCharacterMovement) "MOVE_Walking" 0)
            (goto _label Reset))
          (:else))))))

(event Input|EnhancedActionEvents|EnhancedInputActionia_troca_visao
  (params (ActionValue :type Boolean) (ElapsedSeconds :type Float%20%28double-precision%29) (TriggeredSeconds :type Float%20%28double-precision%29) (InputAction :type Input%20Action%20Object%20Reference :default "/Game/inputs/ia_troca_visao.ia_troca_visao"))
  (bind _springarm (Variables|Camera|GetSpringArm))
  ;[1 1 1] muda camera pra 1ª ou 3ª pessoa (agora com animação)
  (:Started
    (Utilities|FlowControl|FlipFlop
      (:A
        (Audio|PlaySound2D "/Game/sons/fps_ativa.fps_ativa" 1.0 1.0 0.0 0 0)
        (bind (_direction _miraalpha) (Timeline|TimelineCameraVisao Play)
          (:Update
            (Variables|/Script/Engine.SpringArmComponent|SetTargetArmLength _springarm (Math|Float|Lerp 3e+02 -3e+01 _miraalpha))
            (Variables|/Script/Engine.SpringArmComponent|SetTargetOffset _springarm (Math|Vector|Lerp(Vector) "0, 0, 0" "0.000000,0.000000,20.000000" _miraalpha)))
          (:Finished
            (switch Utilities|FlowControl|Switch|SwitchonETimelineDirection _direction
              (:Forward
                (Variables|Default|SetbUseControllerRotationYaw true)
                (Components|Activation|Deactivate (Variables|Camera|GetCamera))
                (Components|Activation|Activate (Variables|Default|GetPrimeiraPessoa) true))))))
      (:B
        (Audio|PlaySound2D "/Game/sons/fps_desativa.fps_desativa" 1.0 1.0 0.0 0 0)
        (Variables|Default|SetbUseControllerRotationYaw false)
        (Components|Activation|Deactivate (Variables|Default|GetPrimeiraPessoa))
        (Components|Activation|Activate (Variables|Camera|GetCamera) true)
        (Timeline|TimelineCameraVisao Reverse)))))

(event Input|EnhancedActionEvents|EnhancedInputActionia_atirar
  (params (ActionValue :type Boolean) (ElapsedSeconds :type Float%20%28double-precision%29) (TriggeredSeconds :type Float%20%28double-precision%29) (InputAction :type Input%20Action%20Object%20Reference :default "/Game/inputs/ia_atirar.ia_atirar"))
  ;[1 1 1] solta um projétil (magia)
  (if (not (Variables|Default|GetGolpeando2))
    (if (Variables|/Game/blueprints/cajado_AC.cajado_AC_C|GetEstáMirando (Actor|GetComponentbyClass "/Game/blueprints/cajado_AC.cajado_AC_C"))
      (Default|TiroComeço (Variables|Default|Getcajado_AC))
      (Variables|Default|SetAtirando true)
      (Utilities|FlowControl|DoOnce false :!label _label
        (:Completed
          (Game|SpawnActorfromClass "/Game/blueprints/magia.magia_C" (Transformation|GetWorldTransform (Variables|Default|Getsai%20o%20tiro)) "Undefined" "MultiplyWithRoot" (Components|GetOwner (Variables|Default|Getcolisão%20cajado%202)) 0 0)
          (Audio|PlaySound2D "/Game/sons/tiro_cajado_2.tiro_cajado_2" 0.9 1.0 0.0 0 0)
          (Utilities|FlowControl|Delay 0.6)
          (Variables|Default|SetAtirando false)
          (goto _label Reset))))))

(event Input|EnhancedActionEvents|EnhancedInputActionia_pausar
  (params (ActionValue :type Boolean) (ElapsedSeconds :type Float%20%28double-precision%29) (TriggeredSeconds :type Float%20%28double-precision%29) (InputAction :type Input%20Action%20Object%20Reference :default "/Game/inputs/ia_pausar.ia_pausar"))
  ;[1 1 1] pausa o jogo
  (bind _returnvalue (UserInterface|CreateWidget "/Game/menus/menu_Pausa.menu_Pausa_C" (Game|GetPlayerController 0)))
  (UserInterface|Viewport|AddtoViewport _returnvalue 2)
  (Audio|PlaySound2D "/Game/sons/pausa.pausa" 1.0 1.0 0.0 0 0))

(event Input|EnhancedActionEvents|EnhancedInputActionia_mirar
  (params (ActionValue :type Boolean) (ElapsedSeconds :type Float%20%28double-precision%29) (TriggeredSeconds :type Float%20%28double-precision%29) (InputAction :type Input%20Action%20Object%20Reference :default "/Game/inputs/ia_mirar.ia_mirar"))
  (bind _cajado_ac (Variables|Default|Getcajado_AC))
  ;[1 1 1] sistema de mira em 3ª pessoa
  (:Started
    (Default|ComeçaMira _cajado_ac)
    (CallFunction|CâmeraMiraComeço)
    (Utilities|IsValid (Variables|Default|GetImagemMIra2)
      (:Is%20Valid
        _)
      (:Is%20Not%20Valid
        (bind _returnvalue (UserInterface|CreateWidget "/Game/ui/mira_ui.mira_ui_C" (Game|GetPlayerController 0)))
        (bind _output_get (Variables|Default|SetImagemMIra2 _returnvalue))))
    (UserInterface|Viewport|AddtoViewport _output_get 1)
    (Variables|/Script/Engine.SpringArmComponent|SetbInheritPitch (Variables|Camera|GetSpringArm) false))
  (:Completed
    (Default|ParaMIra _cajado_ac)
    (CallFunction|CâmeraMiraFim)
    (Widget|RemovefromParent (Variables|Default|GetImagemMIra2))
    (Audio|PlaySound2D "/Game/sons/mira_fim.mira_fim" 1.0 1.0 0.0 0 0)
    (Variables|/Script/Engine.SpringArmComponent|SetbInheritPitch (Variables|Camera|GetSpringArm) true)))

(event EventBeginPlay
  ;[1 1 1] adicionar mapeamento dos botoes
  (bind _asinstancia_intro_musica (Utilities|Casting|CastToinstancia_intro_musica (Game|GetGameInstance)))
  (if (Variables|/Game/blueprints/instancia_intro_musica.instancia_intro_musica_C|GetRodouIntro _asinstancia_intro_musica)
    _
    (else
      ;;[1 1 1] aqui rola a intro
      (Utilities|FlowControl|Delay 6.2)))
  (bind _asplayer_controller (Utilities|Casting|CastToPlayerController (Pawn|GetController)))
  (Utilities|IsValid (PlayerController|LocalPlayerSubsystems|GetEnhancedInputLocalPlayerSubsystem _asplayer_controller)
    (:Is%20Valid
      (Input|AddMappingContext (PlayerController|LocalPlayerSubsystems|GetEnhancedInputLocalPlayerSubsystem _asplayer_controller) "/Game/inputs/imc_protagonista.imc_protagonista" 0 "(bIgnoreAllPressedKeysUntilRelease=True,bForceImmediately=False,bNotifyUserSettings=False)")
      (Variables|Default|SetEstouNoChefe false)
      (Utilities|FlowControl|Sequence
        (:then_0
          (CallFunction|IniciaVariáveis)
          (Utilities|FlowControl|Delay 0.05)
          (for _array_element (Collision|GetOverlappingActors (Variables|Collision|GetCapsuleComponent) "/Game/blueprints/muda_musica_gelo2.muda_musica_gelo2_C" :!class /Script/Engine.PrimitiveComponent)
            (bind _asmuda_musica_gelo_2 (Utilities|Casting|CastTomuda_musica_gelo2 _array_element))
            (Default|MudaMusicaEEscorrega _asmuda_musica_gelo_2)))
        (:then_1
          (Utilities|Time|SetTimerbyEvent (delegate Custom|TocaSomVidaBaixa) 0.05 true)
          (Utilities|Time|SetTimerbyEvent (delegate Custom|atualiza_vida_verm) 0.8 true))
        (:then_2
          (bind _asmodo_de_jogo_principal_alpha (Utilities|Casting|CastTomodoDeJogoPrincipal_alpha (Game|GetGameMode)))
          (Utilities|IsValid (Variables|/Game/blueprints/modoDeJogoPrincipal_alpha.modoDeJogoPrincipal_alpha_C|GetBarraVidaUI _asmodo_de_jogo_principal_alpha)
            (:Is%20Valid
              (Default|AtualizaBarraRed (Variables|/Game/blueprints/modoDeJogoPrincipal_alpha.modoDeJogoPrincipal_alpha_C|GetBarraVidaUI _asmodo_de_jogo_principal_alpha)))))
        (:then_3
          (bind _asinstancia_intro_musica_2 (Utilities|Casting|CastToinstancia_intro_musica (Game|GetGameInstance)))
          (if (Variables|/Game/blueprints/instancia_intro_musica.instancia_intro_musica_C|GetCorAlternativa _asinstancia_intro_musica_2)
            (Rendering|Material|SetMaterial (Variables|Character|GetMesh) 0 "/Game/materiais/new_alpha_mt_alternativo.new_alpha_mt_alternativo")))))))

(fn ConstructionScript
  (bind _bpc_sistema_dano (Variables|Default|Getbpc_sistema_dano))
  (EventDispatchers|BindEventtoNoBloqueio _bpc_sistema_dano (EventDispatchers|CreateEvent :!event Custom|Bloqueou))
  (EventDispatchers|BindEventtoNaRespostaAoDano _bpc_sistema_dano (EventDispatchers|CreateEvent :!event Custom|RespostaAoDano))
  (EventDispatchers|BindEventtoNaMorte _bpc_sistema_dano (EventDispatchers|CreateEvent :!event Custom|Morreu)))

(fn Respawn
  (bind _mesh (Variables|Character|GetMesh))
  (Transformation|SetActorLocationAndRotation (Variables|Default|GetCheckpointLocalAtual) "0.000000,180.000000,0.000000")
  (Variables|/Game/sistema_dano/bpc_sistema_dano.bpc_sistema_dano_C|SetEstáMorto (Variables|Default|Getbpc_sistema_dano) false)
  (CallFunction|Cura 2e+02)
  (Transformation|AttachComponentToComponent (Variables|Camera|GetSpringArm) (Variables|Collision|GetCapsuleComponent) "None" "SnapToTarget" "SnapToTarget" "SnapToTarget" true)
  (Input|EnableInput (Game|GetPlayerController 0))
  (Variables|/Script/Engine.CharacterMovementComponent|SetGravityScale (Variables|Character|GetCharacterMovement) 1.75)
  (Physics|SetSimulatePhysics _mesh false)
  (Collision|SetCollisionEnabled _mesh "QueryOnly")
  (Transformation|AttachComponentToComponent _mesh (Variables|Collision|GetCapsuleComponent) "None" "SnapToTarget" "SnapToTarget" "SnapToTarget" true)
  (Components|Animation|SetAnimationMode _mesh "AnimationBlueprint" true)
  (Transformation|SetRelativeScale3D _mesh "0.185000,0.185000,0.185000")
  (Transformation|SetRelativeLocationAndRotation _mesh "0.000000,0.000000,-91.000000" "0.000000,270.000000,0.000000" false false)
  (Transformation|SetRelativeLocation (Variables|Camera|GetSpringArm) "0.000000,0.000000,31.000000" false false)
  (Rendering|SetVisibility _mesh true true)
  (Utilities|FlowControl|Sequence
    (:then_0
      (bind _asinstancia_intro_musica (Utilities|Casting|CastToinstancia_intro_musica (Game|GetGameInstance)))
      (if (not (<= (Variables|/Game/blueprints/instancia_intro_musica.instancia_intro_musica_C|GetPontos _asinstancia_intro_musica) 499))
        (Default|AdicionaPontuação _asinstancia_intro_musica -500)))
    (:then_1
      (bind _outactors (Actor|GetAllActorsOfClass "/Game/blueprints/chefao_BP_Child.chefao_BP_Child_C"))
      (Utilities|IsValid (Utilities|Array|Get(acopy) _outactors)
        (:Is%20Valid
          (Default|Cura (Variables|/Game/blueprints/inimigo_BP.inimigo_BP_C|Getbpc_sistema_dano (Utilities|Array|Get(acopy) _outactors)) 1e+03))))
    (:then_2
      (bind _asmodo_de_jogo_principal_alpha (Utilities|Casting|CastTomodoDeJogoPrincipal_alpha (Game|GetGameMode)))
      (Default|AtualizaBarraRed (Variables|/Game/blueprints/modoDeJogoPrincipal_alpha.modoDeJogoPrincipal_alpha_C|GetBarraVidaUI _asmodo_de_jogo_principal_alpha)))))

(fn Cura
  (params (Quantidade :type Float%20%28double-precision%29))
  (bind _novavida (Default|Cura (Variables|Default|Getbpc_sistema_dano) Quantidade))
  (return _novavida))

(fn LevaDano
  (params (InfoDano :type S%20Info%20Dano%20Structure))
  (bind _levoudano (Default|LevaDano (Variables|Default|Getbpc_sistema_dano) InfoDano))
  (return _levoudano))

(fn TerVidaAtual
  (return (Variables|/Game/sistema_dano/bpc_sistema_dano.bpc_sistema_dano_C|GetVida (Variables|Default|Getbpc_sistema_dano))))

(fn TerVidaMaxima
  (params (Quantidade :type Float%20%28double-precision%29))
  (return (Variables|/Game/sistema_dano/bpc_sistema_dano.bpc_sistema_dano_C|GetVidaMaxima (Variables|Default|Getbpc_sistema_dano))))