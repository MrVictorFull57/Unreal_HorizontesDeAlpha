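; Main game mode for Stella that builds the player's HUD when play begins.
; It adds the inventory widget immediately, then checks the intro-music game instance and waits about six seconds if the intro has not yet run.
; It then adds a health bar bound to the alpha_BP player character as the damageable actor, along with a points widget.
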(event EventBeginPlay
  (Utilities|FlowControl|Sequence
    (:then_0
      (bind _returnvalue (UserInterface|CreateWidget "/Game/ui/inventario_ui.inventario_ui_C"))
      (UserInterface|Viewport|AddtoViewport _returnvalue 0))
    (:then_1
      (bind _asinstancia_intro_musica (Utilities|Casting|CastToinstancia_intro_musica (Game|GetGameInstance)))
      (if (Variables|/Game/blueprints/instancia_intro_musica.instancia_intro_musica_C|GetRodouIntro _asinstancia_intro_musica)
        _
        (else
          (Utilities|FlowControl|Delay 6.2)))
      (Utilities|FlowControl|Sequence
        (:then_0
          (bind _asalpha_bp (Utilities|Casting|CastToalpha_BP (Game|GetPlayerCharacter 0)))
          (bind _returnvalue_2 (UserInterface|CreateWidget "/Game/ui/barra_de_vida_ui_padrao.barra_de_vida_ui_padrao_C" 0 _asalpha_bp))
          (bind _output_get (Variables|Default|SetBarraVidaUI _returnvalue_2))
          (UserInterface|Viewport|AddtoViewport _output_get 0))
        (:then_1
          (bind _returnvalue_3 (UserInterface|CreateWidget "/Game/ui/pontos_ui.pontos_ui_C"))
          (UserInterface|Viewport|AddtoViewport _returnvalue_3 0))))))

(fn ConstructionScript)