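; Enemy character that forwards damage, healing and health queries to its BpcSistemaDano component and binds that component's block, damage-response and death delegates.
; It registers in the game instance's living-enemy count; block and damage responses only print.
; Being shot (InimigoLevouPipoco) pauses movement for a hit animation with per-actor time-dilation hit-stop.
; Death ragdolls it, then after a delay explodes with camera shake, awards score, decrements the count and destroys it.
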(event Custom|InimigoLevou%20Pipoco
  (bind _mesh (Variables|Character|GetMesh))
  (bind _charactermovement (Variables|Character|GetCharacterMovement))
  (Pawn|Components|CharacterMovement|SetMovementMode _charactermovement "MOVE_None" 0)
  (Components|Animation|PlayAnimation _mesh (Variables|Default|GetOnHit) false)
  (CallFunction|ComeçaHitStop 0.09)
  (Utilities|FlowControl|Delay 1.0)
  (Components|Animation|SetAnimationMode _mesh "AnimationBlueprint" true)
  (Pawn|Components|CharacterMovement|SetMovementMode _charactermovement "MOVE_Walking" 0))

(event Custom|Morreu
  (bind _mesh (Variables|Character|GetMesh))
  (bind _mesh_2 (Variables|Character|GetMesh))
  (bind _returnvalue (Transformation|GetSocketLocation _mesh_2 "Spine"))
  (Variables|Default|Setesta_morto true)
  (Development|PrintString "AE MORREU CARALHO!")
  (Components|Movement|StopMovementImmediately (Variables|Character|GetCharacterMovement))
  (Physics|SetSimulatePhysics _mesh true)
  (Collision|SetCollisionEnabled (Variables|Collision|GetCapsuleComponent) "NoCollision")
  (Collision|SetCollisionEnabled _mesh "PhysicsOnly")
  (Audio|PlaySoundatLocation "/Game/sons/cues/inimigo_morre_cue.inimigo_morre_cue" (Transformation|GetActorLocation) "0, 0, 0" 1.0 1.0 0.0 0 0 0 0)
  (Utilities|FlowControl|Delay 1.5)
  (Effects|SpawnEmitteratLocation "/Game/StarterContent/Particles/P_Explosion.P_Explosion" _returnvalue "0, 0, 0" "1.250000,1.250000,1.250000")
  (Audio|PlaySoundatLocation "/Game/sons/cues/inimigo_explodiu_Cue.inimigo_explodiu_Cue" _returnvalue "0, 0, 0" 1.0 1.0 0.0 0 0 0 0)
  (Camera|PlayWorldCameraShake "/Game/blueprints/ChacoalhaCamera_Inimigo_BP.ChacoalhaCamera_Inimigo_BP_C" (Transformation|GetActorLocation) 0.0 3e+03)
  (bind _asinstancia_intro_musica (Utilities|Casting|CastToinstancia_intro_musica (Game|GetGameInstance)))
  (Default|AdicionaPontuação _asinstancia_intro_musica 250)
  (bind _output_get (Variables|/Game/blueprints/instancia_intro_musica.instancia_intro_musica_C|SetInimigosVivos _asinstancia_intro_musica (- (Variables|/Game/blueprints/instancia_intro_musica.instancia_intro_musica_C|GetInimigosVivos _asinstancia_intro_musica) 1)))
  (Development|PrintString (Utilities|String|ToString(Integer) _output_get))
  (Actor|DestroyActor))

(event Custom|Bloqueou
  (params (PodeDarParry :type Boolean))
  (Development|PrintString "DEU PARRY!"))

(event Custom|RespostaAoDano
  (params (RespostaAoDano :type e_resposta_dano%20Enum :default "NewEnumerator0"))
  (Development|PrintString (Utilities|String|EnumtoString RespostaAoDano)))

(event EventBeginPlay
  (bind _asinstancia_intro_musica (Utilities|Casting|CastToinstancia_intro_musica (Game|GetGameInstance)))
  (bind _output_get (Variables|/Game/blueprints/instancia_intro_musica.instancia_intro_musica_C|SetInimigosVivos _asinstancia_intro_musica (+ (Variables|/Game/blueprints/instancia_intro_musica.instancia_intro_musica_C|GetInimigosVivos _asinstancia_intro_musica) 1)))
  (Development|PrintString (Utilities|String|ToString(Integer) _output_get)))

(fn ConstructionScript
  (bind _bpc_sistema_dano (Variables|Default|Getbpc_sistema_dano))
  (EventDispatchers|BindEventtoNoBloqueio _bpc_sistema_dano (EventDispatchers|CreateEvent :!event Custom|Bloqueou))
  (EventDispatchers|BindEventtoNaRespostaAoDano _bpc_sistema_dano (EventDispatchers|CreateEvent :!event Custom|RespostaAoDano))
  (EventDispatchers|BindEventtoNaMorte _bpc_sistema_dano (EventDispatchers|CreateEvent :!event Custom|Morreu)))

(fn ComeçaHitStop
  (params (Duração :type Float%20%28single-precision%29))
  (Variables|Default|SetCustomTimeDilation 0.05)
  (Utilities|Time|SetTimerbyFunctionName 0 "Termina_Hit_Stop" Duração))

(fn TerminaHitStop
  (Variables|Default|SetCustomTimeDilation 1.0))

(fn Cura
  (params (Quantidade :type Float%20%28double-precision%29))
  (bind _novavida (Default|Cura (Variables|Default|Getbpc_sistema_dano) Quantidade))
  (return _novavida))

(fn LevaDano
  (params (InfoDano :type S%20Info%20Dano%20Structure))
  (bind _levoudano (Default|LevaDano (Variables|Default|Getbpc_sistema_dano) InfoDano))
  (return _levoudano))

(fn TerVidaAtual
  (return (Variables|/Game/sistema_dano/bpc_sistema_dano.bpc_sistema_dano_C|GetVida (Variables|Default|Getbpc_sistema_dano))))

(fn TerVidaMaxima
  (params (Quantidade :type Float%20%28double-precision%29))
  (return (Variables|/Game/sistema_dano/bpc_sistema_dano.bpc_sistema_dano_C|GetVidaMaxima (Variables|Default|Getbpc_sistema_dano))))