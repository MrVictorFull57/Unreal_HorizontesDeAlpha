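; Floating platform actor that travels along an InterpToMovement path, with a sound and a repeating distortion effect.
; The construction script builds a relative path from the origin to LocalMovimento, sets its duration from DuraçãoPlat and applies MaterialPlat to the mesh.
; BeginPlay plays the sound once at the mesh, then starts Brotacalor, a self-calling delayed event that repeatedly spawns the distortion particle at the mesh's current location.
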(event Custom|brotacalor
  (Effects|SpawnEmitteratLocation "/Game/vfx/particulas/distorção_ptc.distorção_ptc" (Transformation|GetWorldLocation (Variables|Default|GetStaticMesh)) "0, 0, 0" "2.000000,2.000000,2.000000")
  (Utilities|FlowControl|Delay 0.5)
  (CallFunction|Brotacalor))

(event EventBeginPlay
  (Audio|PlaySoundatLocation "/Game/sons/plataforma-flutuante.plataforma-flutuante" (Transformation|GetWorldLocation (Variables|Default|GetStaticMesh)) "0, 0, 0" 1.0 1.0 0.0 0 0 0 0)
  (CallFunction|Brotacalor))

(event Collision|EventActorBeginOverlap
  (params (OtherActor :type Actor%20Object%20Reference)))

(event EventTick
  (params (DeltaSeconds :type Float%20%28single-precision%29)))

(fn ConstructionScript
  (bind _interptomovement (Variables|Default|GetInterpToMovement))
  (Class|InterptoMovementComponent|AddControlPointPosition _interptomovement "0, 0, 0" true)
  (Class|InterptoMovementComponent|AddControlPointPosition _interptomovement (Variables|Default|GetLocalMovimento) true)
  (Variables|/Script/Engine.InterpToMovementComponent|SetDuration _interptomovement (Variables|Default|GetDuraçãoPlat))
  (Rendering|Material|SetMaterial (Variables|Default|GetStaticMesh) 0 (Variables|Default|GetMaterialPlat)))