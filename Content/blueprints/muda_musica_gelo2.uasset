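; Ice-area trigger volume that makes the alpha_BP character slide and switches the level music to the ice track.
; Box begin overlap lowers ground friction and walking braking deceleration, then swaps the sound on the first Musica_fase actor's Fase audio component.
; End overlap sets normal movement values and the regular track.
; BeginPlay checks existing overlaps to cover spawning inside, fading the music out before the swap.
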(event OnComponentBeginOverlap(Box)
  (params (OverlappedComponent :type Primitive%20Component%20Object%20Reference) (OtherActor :type Actor%20Object%20Reference) (OtherComp :type Primitive%20Component%20Object%20Reference) (OtherBodyIndex :type Integer) (bFromSweep :type Boolean) (SweepResult :type Hit%20Result%20Structure%20%28by%20ref%29))
  ;[1 1 1] troca pra música da fase de gelo ao entrar na respectiva área e deixa o chão escorregadio
  (bind _asalpha_bp (Utilities|Casting|CastToalpha_BP OtherActor))
  (Utilities|FlowControl|DoOnce false :!label _label
    (:Completed
      (Variables|/Script/Engine.CharacterMovementComponent|SetGroundFriction (Variables|/Script/Engine.Character|GetCharacterMovement _asalpha_bp) 1.0)
      (Variables|/Script/Engine.CharacterMovementComponent|SetBrakingDecelerationWalking (Variables|/Script/Engine.Character|GetCharacterMovement _asalpha_bp) 256.0)
      (bind _outactors (Actor|GetAllActorsOfClass "/Game/blueprints/musica_fase.musica_fase_C"))
      (Audio|Components|Audio|Stop (Variables|/Game/blueprints/musica_fase.musica_fase_C|Getfase (Utilities|Array|Get(acopy) _outactors)))
      (Audio|Components|Audio|SetSound (Variables|/Game/blueprints/musica_fase.musica_fase_C|Getfase (Utilities|Array|Get(acopy) _outactors)) "/Game/musicas/fase_gelo_MS.fase_gelo_MS")
      (Audio|Components|Audio|Play (Variables|/Game/blueprints/musica_fase.musica_fase_C|Getfase (Utilities|Array|Get(acopy) _outactors)) 0.0)
      (goto _label Reset))))

(event OnComponentEndOverlap(Box)
  (params (OverlappedComponent :type Primitive%20Component%20Object%20Reference) (OtherActor :type Actor%20Object%20Reference) (OtherComp :type Primitive%20Component%20Object%20Reference) (OtherBodyIndex :type Integer))
  ;[1 1 1] volta pra música da fase normal ao sair da área de gelo e deixa o chão normal
  (bind _asalpha_bp (Utilities|Casting|CastToalpha_BP OtherActor))
  (Utilities|FlowControl|DoOnce false :!label _label
    (:Completed
      (Variables|/Script/Engine.CharacterMovementComponent|SetGroundFriction (Variables|/Script/Engine.Character|GetCharacterMovement _asalpha_bp) 8.0)
      (Variables|/Script/Engine.CharacterMovementComponent|SetBrakingDecelerationWalking (Variables|/Script/Engine.Character|GetCharacterMovement _asalpha_bp) 2048.0)
      (bind _outactors (Actor|GetAllActorsOfClass "/Game/blueprints/musica_fase.musica_fase_C"))
      (Audio|Components|Audio|Stop (Variables|/Game/blueprints/musica_fase.musica_fase_C|Getfase (Utilities|Array|Get(acopy) _outactors)))
      (Audio|Components|Audio|SetSound (Variables|/Game/blueprints/musica_fase.musica_fase_C|Getfase (Utilities|Array|Get(acopy) _outactors)) "/Game/musicas/fase_qumu_proto.fase_qumu_proto")
      (Audio|Components|Audio|Play (Variables|/Game/blueprints/musica_fase.musica_fase_C|Getfase (Utilities|Array|Get(acopy) _outactors)) 0.0)
      (goto _label Reset))))

(event Custom|muda_musica_e_escorrega
  ;[1 1 1] faz as coisas abaixo se spawnar dentro da área de gelo
  (for _array_element (Collision|GetOverlappingActors (Variables|Default|GetBox) "/Game/blueprints/alpha_BP.alpha_BP_C" :!class /Script/Engine.PrimitiveComponent)
    (bind _asalpha_bp (Utilities|Casting|CastToalpha_BP _array_element))
    (Variables|/Script/Engine.CharacterMovementComponent|SetGroundFriction (Variables|/Script/Engine.Character|GetCharacterMovement _asalpha_bp) 1.0)
    (Variables|/Script/Engine.CharacterMovementComponent|SetBrakingDecelerationWalking (Variables|/Script/Engine.Character|GetCharacterMovement _asalpha_bp) 256.0)
    (bind _outactors (Actor|GetAllActorsOfClass "/Game/blueprints/musica_fase.musica_fase_C"))
    (Audio|Components|Audio|FadeOut (Variables|/Game/blueprints/musica_fase.musica_fase_C|Getfase (Utilities|Array|Get(acopy) _outactors)) 0.3 0.0 "Linear" :!class /Script/Engine.AudioComponent)
    (Utilities|FlowControl|Delay 0.3)
    (Audio|Components|Audio|Stop (Variables|/Game/blueprints/musica_fase.musica_fase_C|Getfase (Utilities|Array|Get(acopy) _outactors)))
    (Audio|Components|Audio|SetSound (Variables|/Game/blueprints/musica_fase.musica_fase_C|Getfase (Utilities|Array|Get(acopy) _outactors)) "/Game/musicas/fase_gelo_MS.fase_gelo_MS")
    (Audio|Components|Audio|Play (Variables|/Game/blueprints/musica_fase.musica_fase_C|Getfase (Utilities|Array|Get(acopy) _outactors)) 0.0)))

(event EventBeginPlay
  ;[1 1 1] faz as coisas abaixo se spawnar dentro da área de gelo
  (CallFunction|MudaMusicaEEscorrega))

(event Collision|EventActorBeginOverlap
  (params (OtherActor :type Actor%20Object%20Reference)))

(event EventTick
  (params (DeltaSeconds :type Float%20%28single-precision%29)))

(fn ConstructionScript)