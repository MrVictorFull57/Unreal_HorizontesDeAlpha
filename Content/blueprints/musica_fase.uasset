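; Level music controller Blueprint that plays the stage track through an audio component and reacts to game events.
; On BeginPlay it waits out the intro the first time, using a game instance flag to start immediately afterwards.
; Custom events stop or restart the track on failure and respawn, lower and muffle it on pause, and apply a low-pass filter underwater.
; A timeline drives a pitch distortion when the music slows.
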(event Custom|PausouJogo
  (bind _fase (Variables|Default|Getfase))
  (Audio|Components|Audio|SetVolumeMultiplier _fase 0.45 :!class /Script/Engine.AudioComponent)
  (Audio|Components|Audio|SetLowPassFilterEnabled _fase true :!class /Script/Engine.AudioComponent)
  (Audio|Components|Audio|SetLowPassFilterFrequency _fase 4.5e+02 :!class /Script/Engine.AudioComponent))

(event Custom|DespausouJogo
  (bind _fase (Variables|Default|Getfase))
  (Audio|Components|Audio|SetVolumeMultiplier _fase 0.9 :!class /Script/Engine.AudioComponent)
  (Audio|Components|Audio|SetLowPassFilterEnabled _fase false :!class /Script/Engine.AudioComponent))

(event Custom|respawnoujogo
  (bind _fase (Variables|Default|Getfase))
  (Audio|Components|Audio|Play _fase 0.0)
  (Audio|Components|Audio|SetPitchMultiplier _fase 1.0))

(event Custom|faliceujogo
  (Audio|Components|Audio|Stop (Variables|Default|Getfase)))

(event Custom|EntrouNaAgua
  (bind _fase (Variables|Default|Getfase))
  (Audio|Components|Audio|SetLowPassFilterEnabled _fase true :!class /Script/Engine.AudioComponent)
  (Audio|Components|Audio|SetLowPassFilterFrequency _fase 8e+02 :!class /Script/Engine.AudioComponent))

(event Custom|MusicaFicouLenta
  (bind _distorção_alpha (Timeline|distorção_tom PlayFromStart)
    (:Update
      (Audio|Components|Audio|SetPitchMultiplier (Variables|Default|Getfase) _distorção_alpha))))

(event EventBeginPlay
  ;[1 1 1] começa a tocar a música da fase apenas após a intro (com um delay), se caso esta já tenha rodado antes, a música começa a tocar instantaneamente
  (bind _asinstancia_intro_musica (Utilities|Casting|CastToinstancia_intro_musica (Game|GetGameInstance)))
  (if (Variables|/Game/blueprints/instancia_intro_musica.instancia_intro_musica_C|GetRodouIntro _asinstancia_intro_musica)
    _
    (else
      (Utilities|FlowControl|Delay 6.2)))
  (Variables|/Game/blueprints/instancia_intro_musica.instancia_intro_musica_C|SetRodouIntro _asinstancia_intro_musica true)
  (Audio|Components|Audio|Play (Variables|Default|Getfase) 0.0))

(fn ConstructionScript)