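; Child Blueprint of the playable character Lana, adding her death, victory and trap-damage reactions.
; Morreu detaches the spring arm, disables input, plays death animation and voice, slows the level music, briefly dips time dilation, then shows Game Over.
; VenceuLevel faces Lana to the camera, blends FOV and boom offset by timeline, fades music and shows the victory menu.
; AreaDano flags damage and briefly halts movement for a hit montage; ForaAreaDano clears the flag.
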(event EventBeginPlay
  (|CallParentFunction))

(event EventMorreu
  ;[1 1 1] morte - lana edition
  (Utilities|FlowControl|DoOnce false :!label _label
    (:Completed
      (Development|PrintString "MORRI, QUE MERDA...")
      (Transformation|DetachFromComponent (Variables|Default|GetSpringArm) "KeepWorld" "KeepWorld" "KeepWorld" true)
      (Input|DisableInput (Game|GetPlayerController 0))
      (Components|Animation|PlayAnimation (Variables|Character|GetMesh) "/Game/animacoes/lana/morre.morre" false)
      (Audio|PlaySoundatLocation "/Game/sons/vozes/lana_voz_morte.lana_voz_morte" (Transformation|GetActorLocation) "0, 0, 0" 1.0 1.0 0.0 0 0 0 0)
      (bind _outactors (Actor|GetAllActorsOfClass "/Game/blueprints/musica_fase.musica_fase_C"))
      (Default|MusicaFicouLenta (Utilities|Array|Get(acopy) _outactors))
      (Utilities|Time|SetGlobalTimeDilation 0.2)
      (Utilities|FlowControl|Delay 0.03)
      (Utilities|Time|SetGlobalTimeDilation 1.0)
      (Utilities|FlowControl|Delay 2.4)
      (Utilities|FlowControl|Delay 1.0)
      (if (not (Variables|Default|GetJáTáMorta))
        (bind _returnvalue (UserInterface|CreateWidget "/Game/menus/menu_GameOver.menu_GameOver_C" (Game|GetPlayerController 0)))
        (Variables|Default|SetJáTáMorta true)
        (UserInterface|Viewport|AddtoViewport _returnvalue 2)
        (goto _label Reset)))))

(event EventVenceuLevel
  (bind _springarm (Variables|Default|GetSpringArm))
  ;[1 1 1] vitória
  (Utilities|FlowControl|Delay 0.8)
  (Input|DisableInput (Game|GetPlayerController 0))
  (Transformation|SetActorRotation (Math|Rotator|FindLookatRotation (Transformation|GetActorLocation) (Transformation|GetWorldLocation (Variables|Default|GetCamera))))
  (bind _miraalpha (Timeline|Timeline_0 Play)
    (:Update
      (Camera|SetFieldOfView (Variables|Default|GetCamera) (Math|Float|Lerp (Variables|Default|GetNormalPOV) (Variables|Default|GetVitoriaPOV) _miraalpha))
      (Variables|/Script/Engine.SpringArmComponent|SetSocketOffset _springarm (Math|Vector|Lerp(Vector) (Variables|Default|GetNormalBoom) (Variables|Default|GetVitoriaBoom) _miraalpha))
      (Variables|/Script/Engine.SpringArmComponent|SetbInheritPitch _springarm false)
      (bind _outactors (Actor|GetAllActorsOfClass "/Game/blueprints/musica_fase.musica_fase_C"))
      (Audio|Components|Audio|FadeOut (Variables|/Game/blueprints/musica_fase.musica_fase_C|Getfase (Utilities|Array|Get(acopy) _outactors)) 1.0 0.0 "Linear" :!class /Script/Engine.AudioComponent)
      (Utilities|FlowControl|Delay 1.0)
      (Audio|Components|Audio|Stop (Variables|/Game/blueprints/musica_fase.musica_fase_C|Getfase (Utilities|Array|Get(acopy) _outactors)))
      (Viewport|RemoveAllWidgets)
      (Components|Animation|PlayAnimation (Variables|Character|GetMesh) "/Game/animacoes/lana/venceu.venceu" false)
      (Audio|PlaySound2D "/Game/musicas/vitória2.vitória2" 1.0 1.0 0.0 0 0)
      (Audio|PlaySoundatLocation "/Game/sons/vozes/lana_voz_venceu.lana_voz_venceu" (Transformation|GetActorLocation) "0, 0, 0" 1.0 1.0 0.0 0 0 0 0)
      (Utilities|FlowControl|Delay 1.0)
      (bind _returnvalue (UserInterface|CreateWidget "/Game/menus/menu_Vitoria.menu_Vitoria_C" (Game|GetPlayerController 0)))
      (UserInterface|Viewport|AddtoViewport _returnvalue 2))))

(event EventAreaDano
  ;[1 1 1] verifica armadilha
  (Variables|Default|SetSofrer_dano true)
  (Utilities|FlowControl|DoOnce false :!label _label
    (:Completed
      (Pawn|Components|CharacterMovement|SetMovementMode (Variables|Character|GetCharacterMovement) "MOVE_None" 0)
      (Animation|PlayAnimMontage (Variables|Default|GetAnimDeLevarDano) 1.0 "None")
      (Utilities|FlowControl|Delay 0.55)
      (Pawn|Components|CharacterMovement|SetMovementMode (Variables|Character|GetCharacterMovement) "MOVE_Walking" 0)
      (goto _label Reset))))

(event EventForaAreaDano
  ;[1 1 1] verifica armadilha
  (Variables|Default|SetSofrer_dano false))

(fn ConstructionScript)