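; Boss-pause component that plays a dramatic hit stop with a camera push toward a target actor.
; A camera spawned at BeginPlay is placed between the target and the player camera, aimed at the target, and blended to.
; Meanwhile, target and attacker freeze via per-actor CustomTimeDilation, leaving the rest of the world running.
; After the delay, dilation resets and the view blends back to the player pawn over that same duration.
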(event Custom|IniciaSequencia
  (params (AtorAlvo :type Actor%20Object%20Reference) (DistanciaAlpha :type Float%20%28single-precision%29) (AtorQueAtaca :type Actor%20Object%20Reference) (DuraçãoParada :type Float%20%28single-precision%29))
  (CallFunction|CameraVaiProChefao AtorAlvo DistanciaAlpha)
  (CallFunction|GerenciaTempo (Utilities|Array|MakeArray AtorAlvo AtorQueAtaca) DuraçãoParada))

(event Custom|GerenciaTempo
  (params (AtoresAfetados :type Array%20of%20Actor%20Object%20References) (DuraçãoParada :type Float%20%28single-precision%29))
  (CallFunction|DefineDilaçãoNosAtores AtoresAfetados 0.0)
  (Utilities|FlowControl|Delay DuraçãoParada)
  (CallFunction|DefineDilaçãoNosAtores AtoresAfetados 1.0)
  (Game|Player|SetViewTargetwithBlend (Game|GetPlayerController 0) (Game|Player|GetPlayerPawn 0) DuraçãoParada "VTBlend_Cubic" 0.0 false))

(event EventBeginPlay
  (bind _returnvalue (Game|SpawnActorfromClass "/Script/Engine.CameraActor" (Math|Transform|MakeTransform "0, 0, 0" "0, 0, 0" "1.000000,1.000000,1.000000") "Undefined" "MultiplyWithRoot" 0 0))
  (bind _output_get (Variables|Default|SetCameraChefao _returnvalue))
  (Class|CameraComponent|SetConstraintAspectRatio (Variables|/Script/Engine.CameraActor|GetCameraComponent _output_get) false))

(fn CameraVaiProChefao
  (params (AtorAlvo :type Actor%20Object%20Reference) (DistanciaAlpha :type Float%20%28single-precision%29))
  (Transformation|SetActorLocation (Variables|Default|GetCameraChefao) (Math|Vector|Lerp(Vector) (Transformation|GetActorLocation AtorAlvo) (Camera|GetCameraLocation (Game|GetPlayerCameraManager 0)) DistanciaAlpha) false false)
  (Transformation|SetActorRotation (Variables|Default|GetCameraChefao) (Math|Rotator|FindLookatRotation (Camera|GetCameraLocation (Game|GetPlayerCameraManager 0)) (Transformation|GetActorLocation AtorAlvo)))
  (Game|Player|SetViewTargetwithBlend (Game|GetPlayerController 0) (Variables|Default|GetCameraChefao) 0.3 "VTBlend_Cubic" 0.0 false))

(fn DefineDilaçãoNosAtores
  (params (AtoresAfetados :type Array%20of%20Actor%20Object%20References) (Dilação :type Float%20%28single-precision%29))
  (for _array_element AtoresAfetados
    (Variables|/Script/Engine.Actor|SetCustomTimeDilation _array_element Dilação))
  (return))