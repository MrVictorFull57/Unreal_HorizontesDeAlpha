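; Fire gate Blueprint: a double door that alpha_BP unlocks with the fire key at the Entrada trigger.
; A one-shot timeline swings both leaves open with sounds, consumes the key and marks the gate as opened.
; Without the key, a Gate and resettable DoOnce show a timed hint widget with audio until the gate has opened.
; The Saida trigger reverses the timeline once to close the doors, and each finished swing plays a slam sound.
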(event OnComponentBeginOverlap(entrada)
  (params (OverlappedComponent :type Primitive%20Component%20Object%20Reference) (OtherActor :type Actor%20Object%20Reference) (OtherComp :type Primitive%20Component%20Object%20Reference) (OtherBodyIndex :type Integer) (bFromSweep :type Boolean) (SweepResult :type Hit%20Result%20Structure%20%28by%20ref%29))
  (bind _returnvalue (Transformation|GetActorLocation))
  (bind _asalpha_bp (Utilities|Casting|CastToalpha_BP OtherActor))
  (if (Variables|/Game/blueprints/alpha_BP.alpha_BP_C|Gettem_chave_fogo _asalpha_bp)
    (Utilities|FlowControl|DoOnce false
      (:Completed
        (bind (_direction _portao_direito _portao_esquerdo) (Timeline|portao_animacao PlayFromStart)
          (:Update
            (Transformation|SetRelativeRotation (Variables|Default|Getportao_d) (Math|Rotator|MakeRotator 0.0 0.0 _portao_direito) false false)
            (Transformation|SetRelativeRotation (Variables|Default|Getportao_e) (Math|Rotator|MakeRotator 0.0 0.0 _portao_esquerdo) false false)
            (Utilities|FlowControl|DoOnce false
              (:Completed
                (Audio|PlaySound2D "/Game/sons/portao_pode_abrir.portao_pode_abrir" 1.0 1.0 0.0 0 0)
                (Audio|PlaySoundatLocation "/Game/sons/portao_destranca.portao_destranca" _returnvalue "0, 0, 0" 1.0 1.0 0.0 0 0 0 0)
                (Variables|/Game/blueprints/alpha_BP.alpha_BP_C|Settem_chave_fogo _asalpha_bp false)
                (Variables|Default|SetPortaoJaAbriu true)
                (Utilities|FlowControl|Delay 0.15)
                (Audio|PlaySoundatLocation "/Game/sons/portao_abrindo.portao_abrindo" _returnvalue "0, 0, 0" 1.0 1.0 0.0 0 0 0 0))))
          (:Finished
            (Audio|PlaySoundatLocation "/Game/sons/portao_estrondo.portao_estrondo" (Transformation|GetActorLocation) "0, 0, 0" 1.0 1.0 0.0 0 0 0 0)
            (goto _label Close)))))
    (elif (not (Variables|Default|GetPortaoJaAbriu))
      (Utilities|FlowControl|Gate false :!label _label
        (:Exit
          (Utilities|FlowControl|DoOnce false :!label _label_2
            (:Completed
              (Audio|PlaySound2D "/Game/sons/portao_nao_abre.portao_nao_abre" 1.0 1.0 0.0 0 0)
              (bind _returnvalue_2 (UserInterface|CreateWidget "/Game/ui/hint_fogo_ui.hint_fogo_ui_C"))
              (UserInterface|Viewport|AddtoViewport _returnvalue_2 0)
              (Utilities|FlowControl|Delay 3.0)
              (Widget|RemovefromParent _returnvalue_2)
              (goto _label_2 Reset))))))))

(event OnComponentBeginOverlap(saida)
  (params (OverlappedComponent :type Primitive%20Component%20Object%20Reference) (OtherActor :type Actor%20Object%20Reference) (OtherComp :type Primitive%20Component%20Object%20Reference) (OtherBodyIndex :type Integer) (bFromSweep :type Boolean) (SweepResult :type Hit%20Result%20Structure%20%28by%20ref%29))
  (bind _returnvalue (Transformation|GetActorLocation))
  (Utilities|Casting|CastToalpha_BP OtherActor)
  (Utilities|FlowControl|DoOnce false
    (:Completed
      (bind (_direction _portao_direito _portao_esquerdo) (Timeline|portao_animacao ReverseFromEnd)
        (:Update
          (Transformation|SetRelativeRotation (Variables|Default|Getportao_d) (Math|Rotator|MakeRotator 0.0 0.0 _portao_direito) false false)
          (Transformation|SetRelativeRotation (Variables|Default|Getportao_e) (Math|Rotator|MakeRotator 0.0 0.0 _portao_esquerdo) false false)
          (Utilities|FlowControl|DoOnce false
            (:Completed
              (Audio|PlaySound2D "/Game/sons/portao_pode_abrir.portao_pode_abrir" 1.0 1.0 0.0 0 0)
              (Audio|PlaySoundatLocation "/Game/sons/portao_destranca.portao_destranca" _returnvalue "0, 0, 0" 1.0 1.0 0.0 0 0 0 0)
              (Variables|/Game/blueprints/alpha_BP.alpha_BP_C|Settem_chave_fogo (stale OnComponentBeginOverlap(entrada) _asalpha_bp) false)
              (Variables|Default|SetPortaoJaAbriu true)
              (Utilities|FlowControl|Delay 0.15)
              (Audio|PlaySoundatLocation "/Game/sons/portao_abrindo.portao_abrindo" _returnvalue "0, 0, 0" 1.0 1.0 0.0 0 0 0 0))))
        (:Finished
          (Audio|PlaySoundatLocation "/Game/sons/portao_estrondo.portao_estrondo" (Transformation|GetActorLocation) "0, 0, 0" 1.0 1.0 0.0 0 0 0 0)
          (Utilities|FlowControl|Gate false) ; enters at Close
        )))))

(fn ConstructionScript)