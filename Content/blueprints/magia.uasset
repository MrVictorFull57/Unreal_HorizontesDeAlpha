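; Magic projectile actor that damages an inimigo_BP enemy on contact.
; It emits spark particles on spawn and larger ones when destroyed, and self-destructs after a short delay.
; Box, sphere and actor hits destroy it; box and actor hits also play an impact sound, and box hits call NoImpactoDoProjetil.
; Box overlap with a living enemy applies damage once through LevaDano, triggers InimigoLevouPipoco, then destroys the projectile.
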(event OnComponentBeginOverlap(Box)
  (params (OverlappedComponent :type Primitive%20Component%20Object%20Reference) (OtherActor :type Actor%20Object%20Reference) (OtherComp :type Primitive%20Component%20Object%20Reference) (OtherBodyIndex :type Integer) (bFromSweep :type Boolean) (SweepResult :type Hit%20Result%20Structure%20%28by%20ref%29))
  (bind _asinimigo_bp (Utilities|Casting|CastToinimigo_BP OtherActor))
  (if (not (Variables|/Game/blueprints/inimigo_BP.inimigo_BP_C|Getesta_morto _asinimigo_bp))
    (Utilities|FlowControl|DoOnce false
      (:Completed
        (Default|LevaDano _asinimigo_bp (Utilities|Struct|Makes_info_dano 25.0 "NewEnumerator1"))
        (Default|InimigoLevouPipoco _asinimigo_bp)
        (Actor|DestroyActor)))))

(event OnComponentHit(Box)
  (params (HitComponent :type Primitive%20Component%20Object%20Reference) (OtherActor :type Actor%20Object%20Reference) (OtherComp :type Primitive%20Component%20Object%20Reference) (NormalImpulse :type Vector :default "0, 0, 0") (Hit :type Hit%20Result%20Structure%20%28by%20ref%29))
  (Default|CallNoImpactoDoProjetil OtherActor Hit)
  (Audio|SpawnSoundatLocation (Variables|Default|Getsom_de_impacto) (.Location (Collision|BreakHitResult Hit)) "0, 0, 0" 1.0 1.0 0.0 0 0)
  (Actor|DestroyActor))

(event OnComponentHit(Sphere)
  (params (HitComponent :type Primitive%20Component%20Object%20Reference) (OtherActor :type Actor%20Object%20Reference) (OtherComp :type Primitive%20Component%20Object%20Reference) (NormalImpulse :type Vector :default "0, 0, 0") (Hit :type Hit%20Result%20Structure%20%28by%20ref%29))
  (Actor|DestroyActor))

(event Collision|EventHit
  (params (MyComp :type Primitive%20Component%20Object%20Reference) (Other :type Actor%20Object%20Reference) (OtherComp :type Primitive%20Component%20Object%20Reference) (bSelfMoved :type Boolean) (HitLocation :type Vector :default "0, 0, 0") (HitNormal :type Vector :default "0, 0, 0") (NormalImpulse :type Vector :default "0, 0, 0") (Hit :type Hit%20Result%20Structure%20%28by%20ref%29))
  (Audio|SpawnSoundatLocation (Variables|Default|Getsom_de_impacto) HitLocation "0, 0, 0" 1.0 1.0 0.0 "/Game/sons/atenuação_sons.atenuação_sons" 0)
  (Actor|DestroyActor))

(event EventBeginPlay
  (Effects|SpawnEmitteratLocation "/Game/vfx/particulas/faicas_impacto_ptc.faicas_impacto_ptc" (Transformation|GetWorldLocation (Variables|Default|GetSphere)) "0, 0, 0" "0.500000,0.500000,0.500000")
  (Utilities|FlowControl|Delay 0.7)
  (Actor|DestroyActor))

(event EventDestroyed
  (Effects|SpawnEmitteratLocation "/Game/vfx/particulas/faicas_impacto_ptc.faicas_impacto_ptc" (Transformation|GetActorLocation) "0, 0, 0" "1.500000,1.500000,1.500000"))

(fn ConstructionScript)