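; Health pot pickup that heals the player character (alpha_BP) on overlap.
; The mesh bobs continuously through two looping eased MoveComponentTo moves.
; When Sensor_pote overlaps alpha_BP with Vida at or below a near-full threshold in its damage-system component, it calls CuraMessage, plays particle and sound feedback, then destroys itself.
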(event OnComponentBeginOverlap(sensor_pote)
  (params (OverlappedComponent :type Primitive%20Component%20Object%20Reference) (OtherActor :type Actor%20Object%20Reference) (OtherComp :type Primitive%20Component%20Object%20Reference) (OtherBodyIndex :type Integer) (bFromSweep :type Boolean) (SweepResult :type Hit%20Result%20Structure%20%28by%20ref%29))
  (bind _asalpha_bp (Utilities|Casting|CastToalpha_BP OtherActor))
  (Math|Float|CompareFloat (Variables|/Game/sistema_dano/bpc_sistema_dano.bpc_sistema_dano_C|GetVida (Variables|/Game/blueprints/alpha_BP.alpha_BP_C|Getbpc_sistema_dano _asalpha_bp)) 99.0
    (:==
      _)
    (:<
      _))
  (Class|BpiSistemaDano|Cura(Message) _asalpha_bp 5e+01)
  (Effects|SpawnEmitteratLocation "/Game/vfx/particulas/vida_ptc.vida_ptc" (Transformation|GetActorLocation))
  (Audio|PlaySound2D "/Game/sons/recupera_vida.recupera_vida" 1.0 1.0 0.0 0 0)
  (Actor|DestroyActor))

(event EventBeginPlay
  (bind _staticmesh (Variables|Default|GetStaticMesh))
  (Components|MoveComponentTo _staticmesh "0.000000,0.000000,50.000000" "0, 0, 0" true true 2.5 false :!label _label)
  (Components|MoveComponentTo _staticmesh "0, 0, 0" "0, 0, 0" true true 2.5 false)
  (goto _label))

(fn ConstructionScript)