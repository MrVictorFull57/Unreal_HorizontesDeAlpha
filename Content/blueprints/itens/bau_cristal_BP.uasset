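; Crystal chest that the player (alpha_BP) can open once to earn points.
; Sensor overlaps tell the player it is in range and toggle the Aviso prompt.
; The externally triggered anim_abrir_bau disables the sensor, plays the chest animation and reveals the crystal, which a timeline moves and spins.
; A DoOnce on that timeline's update plays a sound, then after a delay bursts particles, destroys the crystal and adds score through the game instance.
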(event OnComponentBeginOverlap(sensor)
  (params (OverlappedComponent :type Primitive%20Component%20Object%20Reference) (OtherActor :type Actor%20Object%20Reference) (OtherComp :type Primitive%20Component%20Object%20Reference) (OtherBodyIndex :type Integer) (bFromSweep :type Boolean) (SweepResult :type Hit%20Result%20Structure%20%28by%20ref%29))
  ;[1 1 1] ligar ou desligar se está na área
  (bind _asalpha_bp (Utilities|Casting|CastToalpha_BP OtherActor))
  (Default|EstaNaArea _asalpha_bp self)
  (if (not (Variables|Default|GetBauJáAbriu))
    (Rendering|SetVisibility (Variables|Default|Getaviso) true false)))

(event OnComponentEndOverlap(sensor)
  (params (OverlappedComponent :type Primitive%20Component%20Object%20Reference) (OtherActor :type Actor%20Object%20Reference) (OtherComp :type Primitive%20Component%20Object%20Reference) (OtherBodyIndex :type Integer))
  ;[1 1 1] ligar ou desligar se está na área
  (bind _asalpha_bp (Utilities|Casting|CastToalpha_BP OtherActor))
  (Default|NaoEstaNaArea _asalpha_bp self)
  (Rendering|SetVisibility (Variables|Default|Getaviso) false false))

(event Custom|anim_abrir_bau
  (bind _cristal (Variables|Default|Getcristal))
  (bind _cristal_2 (Variables|Default|Getcristal))
  ;[1 1 1] abre o baú
  (Collision|SetCollisionEnabled (Variables|Default|Getsensor) "NoCollision")
  (Audio|Components|Audio|Play (Variables|Default|Getbau) false)
  (Variables|Default|SetBauJáAbriu true)
  (Rendering|SetVisibility _cristal true false)
  (bind _movimento_do_cristal (Timeline|cristal_anim Play)
    (:Update
      (Transformation|SetWorldLocation _cristal (+ (Transformation|GetWorldLocation _cristal) _movimento_do_cristal) false false)
      (Transformation|SetWorldRotation _cristal (Math|Rotator|MakeRotator 0.0 0.0 (+ (.yaw (Transformation|GetWorldRotation _cristal)) 4.0)) false false)
      (Utilities|FlowControl|DoOnce false
        (:Completed
          (Audio|PlaySound2D "/Game/sons/pega_item3.pega_item3" 1.0 1.0 0.0 0 0)
          (Utilities|FlowControl|Delay 2.0)
          (Effects|SpawnEmitteratLocation "/Game/vfx/particulas/faicas_impacto_ptc.faicas_impacto_ptc" (Transformation|GetWorldLocation _cristal_2) "0, 0, 0" "2.000000,2.000000,2.000000")
          (Components|DestroyComponent _cristal_2)
          (bind _asinstancia_intro_musica (Utilities|Casting|CastToinstancia_intro_musica (Game|GetGameInstance)))
          (Default|AdicionaPontuação _asinstancia_intro_musica 500))))))

(event EventBeginPlay
  (Variables|Default|SetBauJáAbriu false))

(fn ConstructionScript)