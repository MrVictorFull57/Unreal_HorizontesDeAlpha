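; Fire key pickup that animates its mesh and is collected when alpha_BP overlaps its collision component.
; Two timelines hand off to each other in an endless loop to move the mesh's relative location, the second playing in reverse.
; On pickup it sets the player's TemChaveFogo flag, plays a sound, destroys itself, spawns a spark effect and adds score through the game instance.
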(event OnComponentBeginOverlap(colisao_chave_fogo)
  (params (OverlappedComponent :type Primitive%20Component%20Object%20Reference) (OtherActor :type Actor%20Object%20Reference) (OtherComp :type Primitive%20Component%20Object%20Reference) (OtherBodyIndex :type Integer) (bFromSweep :type Boolean) (SweepResult :type Hit%20Result%20Structure%20%28by%20ref%29))
  (bind _asalpha_bp (Utilities|Casting|CastToalpha_BP OtherActor))
  (Variables|/Game/blueprints/alpha_BP.alpha_BP_C|Settem_chave_fogo _asalpha_bp true)
  (Audio|PlaySound2D "/Game/sons/cues/pega_chave_fogo.pega_chave_fogo" 1.0 1.0 0.0 0 0)
  (Actor|DestroyActor)
  (Effects|SpawnEmitteratLocation "/Game/vfx/particulas/faicas_impacto_ptc.faicas_impacto_ptc" (Transformation|GetActorLocation) "0, 0, 0" "2.000000,2.000000,2.000000")
  (bind _asinstancia_intro_musica (Utilities|Casting|CastToinstancia_intro_musica (Game|GetGameInstance)))
  (Default|AdicionaPontuação _asinstancia_intro_musica 250))

(event EventBeginPlay
  (bind _move (Timeline|Timeline Play)
    (:Update
      (Transformation|SetRelativeLocation (Variables|Default|GetStaticMesh) _move false false))
    (:Finished
      (bind _move_e_roda (Timeline|Timeline_0 ReverseFromEnd)
        (:Update
          (Transformation|SetRelativeLocation (Variables|Default|GetStaticMesh) _move_e_roda false false))
        (:Finished
          (Timeline|Timeline PlayFromStart))))))

(fn ConstructionScript)