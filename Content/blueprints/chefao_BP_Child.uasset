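; Child Blueprint of a boss (chefão) that handles its death and the resulting level victory through the Morreu event.
; Death triggers ragdoll, a brief time-dilation slowdown, music stop and widget clearing, then a delayed explosion with camera shake and actor destruction.
; It then adds score, unlocks phase 2 and the time-stop power in the game instance, saves, shows the power's UI when newly granted, and calls VenceuLevel on the player.
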(event EventMorreu
  (bind _returnvalue (Game|GetPlayerController 0))
  (bind _mesh (Variables|Character|GetMesh))
  (bind _mesh_2 (Variables|Character|GetMesh))
  (bind _returnvalue_2 (Transformation|GetSocketLocation _mesh_2 "Spine"))
  (Variables|Default|Setesta_morto true)
  (Development|PrintString "AE MORREU CARALHO!")
  (Components|Movement|StopMovementImmediately (Variables|Character|GetCharacterMovement))
  (Physics|SetSimulatePhysics _mesh true)
  (Collision|SetCollisionEnabled _mesh "PhysicsOnly")
  (Audio|PlaySoundatLocation "/Game/sons/cues/chefe_morre_cue.chefe_morre_cue" (Transformation|GetActorLocation) "0, 0, 0" 1.0 1.0 0.0 0 0 0 0)
  (Utilities|Time|SetGlobalTimeDilation 0.2)
  (Utilities|FlowControl|Delay 0.03)
  (Utilities|Time|SetGlobalTimeDilation 1.0)
  (bind _outactors (Actor|GetAllActorsOfClass "/Game/blueprints/musica_fase.musica_fase_C"))
  (Audio|Components|Audio|Stop (Variables|/Game/blueprints/musica_fase.musica_fase_C|Getfase (Utilities|Array|Get(acopy) _outactors)))
  (Viewport|RemoveAllWidgets)
  (Utilities|FlowControl|Delay 2.5)
  (Effects|SpawnEmitteratLocation "/Game/StarterContent/Particles/P_Explosion.P_Explosion" _returnvalue_2 "0, 0, 0" "3.000000,3.000000,3.000000")
  (Audio|PlaySoundatLocation "/Game/sons/chefe_explodiu.chefe_explodiu" _returnvalue_2 "0, 0, 0" 1.0 1.0 0.0 0 0 0 0)
  (Camera|PlayWorldCameraShake "/Game/blueprints/ChacoalhaCamera_Chefao_BP.ChacoalhaCamera_Chefao_BP_C" (Transformation|GetActorLocation) 0.0 3e+03)
  (Actor|DestroyActor)
  (Utilities|FlowControl|Sequence
    (:then_0
      (bind _asinstancia_intro_musica (Utilities|Casting|CastToinstancia_intro_musica (Game|GetGameInstance)))
      (Default|AdicionaPontuação _asinstancia_intro_musica 1000)
      (if (Variables|/Game/blueprints/instancia_intro_musica.instancia_intro_musica_C|GetFase2Liberada _asinstancia_intro_musica)
        (Default|SalvaProgresso _asinstancia_intro_musica :!label _label)
        (else
          (Variables|/Game/blueprints/instancia_intro_musica.instancia_intro_musica_C|SetFase2Liberada _asinstancia_intro_musica true)
          (if (Variables|/Game/blueprints/instancia_intro_musica.instancia_intro_musica_C|GetPoder_PararTempo _asinstancia_intro_musica)
            (goto _label)
            (else
              (Variables|/Game/blueprints/instancia_intro_musica.instancia_intro_musica_C|SetPoder_PararTempo _asinstancia_intro_musica true)
              (Default|SalvaProgresso _asinstancia_intro_musica)
              (bind _returnvalue_3 (UserInterface|CreateWidget "/Game/ui/poder_tempo_ui.poder_tempo_ui_C" _returnvalue))
              (UserInterface|Viewport|AddtoViewport _returnvalue_3 2)
              (Input|SetInputModeUIOnly _returnvalue _returnvalue_3 "DoNotLock" false)
              (Variables|/Script/Engine.PlayerController|SetbShowMouseCursor _returnvalue false))))))
    (:then_1
      (bind _asalpha_bp (Utilities|Casting|CastToalpha_BP (Game|GetPlayerCharacter 0)))
      (Default|VenceuLevel _asalpha_bp))))

(fn ConstructionScript
  (|CallParentFunction))