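; Checkpoint trigger actor that records a respawn-style location and rotation on the alpha_BP character when it overlaps the Box.
; Each overlap stores the character's own current transform values in its checkpoint variables, rather than those of the checkpoint actor.
; A DoOnce limits the feedback to the first activation: a 2D sound and a Checkpoint_ui widget shown briefly, then removed after a delay.
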(event OnComponentBeginOverlap(Box)
  (params (OverlappedComponent :type Primitive%20Component%20Object%20Reference) (OtherActor :type Actor%20Object%20Reference) (OtherComp :type Primitive%20Component%20Object%20Reference) (OtherBodyIndex :type Integer) (bFromSweep :type Boolean) (SweepResult :type Hit%20Result%20Structure%20%28by%20ref%29))
  (bind _asalpha_bp (Utilities|Casting|CastToalpha_BP OtherActor))
  (Variables|/Game/blueprints/alpha_BP.alpha_BP_C|SetCheckpointLocalAtual _asalpha_bp (Transformation|GetActorLocation _asalpha_bp))
  (Variables|/Game/blueprints/alpha_BP.alpha_BP_C|SetCheckpointRotaçãoAtual _asalpha_bp (Transformation|GetActorRotation _asalpha_bp))
  (Utilities|FlowControl|DoOnce false
    (:Completed
      (Audio|PlaySound2D "/Game/sons/checkpoint.checkpoint" 1.0 1.0 0.0 0 0)
      (bind _returnvalue (UserInterface|CreateWidget "/Game/ui/checkpoint_ui.checkpoint_ui_C" (Game|GetPlayerController 0)))
      (bind _output_get (Variables|Default|Setcheckpoint_ui _returnvalue))
      (UserInterface|Viewport|AddtoViewport _output_get 2)
      (Utilities|FlowControl|Delay 2.0)
      (Widget|RemovefromParent _output_get))))

(fn ConstructionScript)