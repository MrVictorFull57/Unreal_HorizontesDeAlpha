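; Damage system Blueprint component that tracks an actor's health (Vida), healing and death.
; LevaDano runs each hit's InfoDano through the Dash macro, which sorts it into blocked, damaged or no damage from death, immunity and blocking state.
; Calls report blocks with parry eligibility, death, or a damage response when the hit can interrupt.
; Cura adds clamped health only while alive.
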(event EventBeginPlay)

(event EventTick
  (params (DeltaSeconds :type Float%20%28single-precision%29)))

(fn Cura
  (params (Quantidade :type Float%20%28double-precision%29))
  (if (not (Variables|Default|GetEstáMorto))
    (bind _output_get (Variables|Default|SetVida (Math|Float|Clamp(Float) (+ Quantidade (Variables|Default|GetVida)) 0.0 (Variables|Default|GetVidaMaxima))))
    (return _output_get)))

(fn LevaDano
  (params (InfoDano :type S%20Info%20Dano%20Structure))
  (bind (_quantidade _tipodano _respostadano _estáimuneaodano _podeinterromperaforça _podebloqueardano _podedarparryemdano) (Utilities|Struct|Breaks_info_dano InfoDano))
  (Utilities|Dash _estáimuneaodano _podebloqueardano
    (:BloqueiaDano
      (Default|CallNoBloqueio _podedarparryemdano)
      (return false))
    (:ComDano
      (bind _output_get (Variables|Default|SetVida (- (Variables|Default|GetVida) _quantidade)))
      (if (<= _output_get 0.0)
        (Variables|Default|SetEstáMorto true)
        (Default|CallNaMorte)
        (return true)
        (elif (or (Variables|Default|GetEstáInterrompendo) _podeinterromperaforça)
          (Default|CallNaRespostaAoDano _respostadano)
          (return true))))
    (:SemDano
      (return false))))